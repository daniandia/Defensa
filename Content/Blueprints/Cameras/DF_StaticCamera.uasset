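; DF_StaticCamera is a camera actor that follows a reference actor at a fixed world-space offset.
; IAmTheFollowReference registers the target, stores the camera's current offset from it and switches following on.
; Each Tick, UpdateFollowPlayer teleports the camera component to the target location plus that offset, without changing rotation, and prints the new position for debugging.
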(event `self.ReceiveBeginPlay`)

(event `self.ReceiveTick`
  (params (DeltaSeconds :type "Float (single-precision)"))
  (`self.UpdateFollowPlayer`))

(fn `IAmTheFollowReference`
  (params (NewParam :type "Actor Object Reference"))
  (bind _output_get (set `self.FollowReference` NewParam))
  (bind _output_get_2 (set `self.VectorToPlayer` (- (`SceneComponent.K2_GetComponentLocation` (`self.CameraComponent`)) (`self.K2_GetActorLocation` _output_get))))
  (set `self.MustFollow` true))

(fn `UpdateFollowPlayer`
  (bind _returnvalue (+ (`self.K2_GetActorLocation` (`self.FollowReference`)) (`self.VectorToPlayer`)))
  (if (`self.MustFollow`)
    (`SceneComponent.K2_SetWorldLocation` (`self.CameraComponent`) _returnvalue false true)
    (`KismetSystemLibrary.PrintString` (`KismetStringLibrary.Conv_VectorToString` _returnvalue))))

(fn `UserConstructionScript`)