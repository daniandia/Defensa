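; Player Paper2D character for a side-view game, with run, dodge, jump, double jump, block and a throwable monkey companion.
; An enum state machine drives it: Enhanced Input events request states, each state sets a flipbook, and finished flipbooks or Tick advance transitions.
; Tick also resets rotation and flips sprite scale by velocity to set facing.
; Throwing swaps the carried monkey sprite for the MK_MonkeyChar actor, and capsule contact retrieves it.
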(event `self.ReceiveBeginPlay`
  (`self.K2_SetActorLocationAndRotation` (0.0 0.0 0.0) (struct) false true)
  (`self.InitMappingContext`)
  (bind _returnvalue (`GameplayStatics.GetActorOfClass` "/Game/Blueprints/Cameras/DF_StaticCamera.DF_StaticCamera_C"))
  (`/Game/Blueprints/Cameras/DF_StaticCamera.IAmTheFollowReference` _returnvalue self)
  (bind _returnvalue_2 (`GameplayStatics.GetActorOfClass` "/Game/Blueprints/Characters/Monkey/MK_MonkeyChar.MK_MonkeyChar_C"))
  (set `self.MonkeyReference` _returnvalue_2))

(event `self.ReceiveTick`
  (params (DeltaSeconds :type "Float (single-precision)"))
  ;[1 1 1] DANI: Rot not init propperly (DK What happens)
  (`self.K2_SetActorRotation` (struct))
  (`self.UpdateSpriteScale`)
  (`self.FSMUpdateState`))

(event `EnhancedInput|/Game/Inputs/MainChar/IA_MC_Move`
  (params (ActionValue :type "Float (double-precision)") (ElapsedSeconds :type "Float (double-precision)") (TriggeredSeconds :type "Float (double-precision)") (InputAction :type "InputAction Object Reference" :default "/Game/Inputs/MainChar/IA_MC_Move.IA_MC_Move"))
  (bind _charactermovement (`self.CharacterMovement`))
  (bind _charactermovement_2 (`self.CharacterMovement`))
  (bind _charactermovement_3 (`self.CharacterMovement`))
  (bind _returnvalue (* ActionValue (`self.WalkSpeed`)))
  (bind (_velocity_x _velocity_y) (`KismetMathLibrary.BreakVector` (`MovementComponent.Velocity` _charactermovement)))
  (bind (_velocity_x_2 _velocity_y_2 _velocity_z) (`KismetMathLibrary.BreakVector` (`MovementComponent.Velocity` _charactermovement_2)))
  (bind (_velocity_x_3 _velocity_y_3 _velocity_z_2) (`KismetMathLibrary.BreakVector` (`MovementComponent.Velocity` _charactermovement_3)))
  (:`Triggered`
    (if (!= (`self.LastMoveInputValue`) ActionValue)
      (switch `/Game/Blueprints/Characters/MainChar/DF_MC_FSM_States` (`self.FSM_State`)
        (:`NewEnumerator3`
          (`self.FSMChangeState` "NewEnumerator6")
          (set `MovementComponent.Velocity` (0.0 0.0 0.0) (`self.CharacterMovement`))))
      (else
        (set `self.LastMoveInputValue` ActionValue :!label _label)
        (switch `/Game/Blueprints/Characters/MainChar/DF_MC_FSM_States` (`self.FSM_State`)
          (:`NewEnumerator0`
            (set `MovementComponent.Velocity` (`KismetMathLibrary.MakeVector` _returnvalue 0.0 _velocity_z_2) _charactermovement_3 :!label _label_2)
            (`self.FSMChangeState` "NewEnumerator1"))
          (:`NewEnumerator1`
            (goto _label_2))
          (:`NewEnumerator2`
            (set `MovementComponent.Velocity` (`KismetMathLibrary.MakeVector` _returnvalue 0.0 _velocity_z) _charactermovement_2 :!label _label_3)
            (`self.FSMChangeState` "NewEnumerator3"))
          (:`NewEnumerator3`
            (goto _label_3))))))
  (:`Started`
    (goto _label))
  (:`Completed`
    (set `self.LastMoveInputValue` 0.0)
    (switch `/Game/Blueprints/Characters/MainChar/DF_MC_FSM_States` (`self.FSM_State`)
      (:`NewEnumerator1`
        (set `MovementComponent.Velocity` (0.0 0.0 0.0) (`self.CharacterMovement`))
        (`self.FSMChangeState` "NewEnumerator0"))
      (:`NewEnumerator3`
        (set `MovementComponent.Velocity` (`KismetMathLibrary.MakeVector` 0.0 0.0 _velocity_y) _charactermovement)
        (`self.FSMChangeState` "NewEnumerator5")))))

(event `EnhancedInput|/Game/Inputs/MainChar/IA_MC_Dodge`
  (params (ActionValue :type Boolean) (ElapsedSeconds :type "Float (double-precision)") (TriggeredSeconds :type "Float (double-precision)") (InputAction :type "InputAction Object Reference" :default "/Game/Inputs/MainChar/IA_MC_Dodge.IA_MC_Dodge"))
  (:`Started`
    (switch `/Game/Blueprints/Characters/MainChar/DF_MC_FSM_States` (`self.FSM_State`)
      (:`NewEnumerator2`
        (`self.FSMChangeState` "NewEnumerator4"))
      (:`NewEnumerator3`
        (`self.FSMChangeState` "NewEnumerator7")))))

(event `EnhancedInput|/Game/Inputs/MainChar/IA_MC_FightPose`
  (params (ActionValue :type Boolean) (ElapsedSeconds :type "Float (double-precision)") (TriggeredSeconds :type "Float (double-precision)") (InputAction :type "InputAction Object Reference" :default "/Game/Inputs/MainChar/IA_MC_FightPose.IA_MC_FightPose"))
  (:`Started`
    (switch `/Game/Blueprints/Characters/MainChar/DF_MC_FSM_States` (`self.FSM_State`)
      (:`NewEnumerator2`
        (`self.FSMChangeState` "NewEnumerator8"))))
  (:`Canceled`
    (switch `/Game/Blueprints/Characters/MainChar/DF_MC_FSM_States` (`self.FSM_State`) :!label _label_4
      (:`NewEnumerator8`
        (`self.FSMChangeState` "NewEnumerator2"))))
  (:`Completed`
    (goto _label_4)))

(event `EnhancedInput|/Game/Inputs/MainChar/IA_MV_Block`
  (params (ActionValue :type Boolean) (ElapsedSeconds :type "Float (double-precision)") (TriggeredSeconds :type "Float (double-precision)") (InputAction :type "InputAction Object Reference" :default "/Game/Inputs/MainChar/IA_MV_Block.IA_MV_Block"))
  (:`Started`
    (switch `/Game/Blueprints/Characters/MainChar/DF_MC_FSM_States` (`self.FSM_State`)
      (:`NewEnumerator8`
        (`self.FSMChangeState` "NewEnumerator11")))))

(event `EnhancedInput|/Game/Inputs/MainChar/IA_MC_MonkeySwitch`
  (params (ActionValue :type Boolean) (ElapsedSeconds :type "Float (double-precision)") (TriggeredSeconds :type "Float (double-precision)") (InputAction :type "InputAction Object Reference" :default "/Game/Inputs/MainChar/IA_MC_MonkeySwitch.IA_MC_MonkeySwitch"))
  (:`Started`
    (switch `/Game/Blueprints/Characters/MainChar/DF_MC_FSM_States` (`self.FSM_State`)
      (:`NewEnumerator0`
        (`self.FSMChangeState` "NewEnumerator2"))
      (:`NewEnumerator2`
        (`self.FSMChangeState` "NewEnumerator0")))))

(event `EnhancedInput|/Game/Inputs/MainChar/IA_MC_Jump`
  (params (ActionValue :type Boolean) (ElapsedSeconds :type "Float (double-precision)") (TriggeredSeconds :type "Float (double-precision)") (InputAction :type "InputAction Object Reference" :default "/Game/Inputs/MainChar/IA_MC_Jump.IA_MC_Jump"))
  (:`Started`
    (switch `/Game/Blueprints/Characters/MainChar/DF_MC_FSM_States` (`self.FSM_State`)
      (:`NewEnumerator2`
        (`self.Jump` :!label _label_5)
        (`self.FSMChangeState` "NewEnumerator14"))
      (:`NewEnumerator3`
        (goto _label_5))
      (:`NewEnumerator10`
        (if (`self.CanDoubleJump`)
          (`self.FSMChangeState` "NewEnumerator15")
          (set `self.CanDoubleJump` false))))))

(event `EnhancedInput|/Game/Inputs/MainChar/IA_MV_MonkeyThrow`
  (params (ActionValue :type Boolean) (ElapsedSeconds :type "Float (double-precision)") (TriggeredSeconds :type "Float (double-precision)") (InputAction :type "InputAction Object Reference" :default "/Game/Inputs/MainChar/IA_MV_MonkeyThrow.IA_MV_MonkeyThrow"))
  (:`Started`
    (`self.ThrowMonkey`)))

(event `self.Sprite.OnFinishedPlaying`
  (`self.FlipbookFinishedPlaying`))

(event `self.CapsuleComponent.OnComponentHit`
  (params (HitComponent :type "PrimitiveComponent Object Reference") (OtherActor :type "Actor Object Reference") (OtherComp :type "PrimitiveComponent Object Reference") (NormalImpulse :type "Vector Structure") (Hit :type "HitResult Structure (by ref)"))
  (if (== (`GameplayStatics.GetObjectClass` OtherActor) "/Game/Blueprints/Characters/Monkey/MK_MonkeyChar.MK_MonkeyChar_C")
    (`self.GetMonkey`)))

(fn `BeingAttacked`
  (returns (HitSuccess :type Boolean))
  (return (`|EnumEquality` (`self.FSM_State`) "NewEnumerator11")))

(fn `FlipbookFinishedPlaying`
  (bind _returnvalue (`|GetInputActionValue`))
  (bind _fsm_state (`self.FSM_State`))
  (`KismetSystemLibrary.PrintString` (`KismetStringLibrary.Concat_StrStr` "ANIM FINISHED : " (`|GetEnumeratorNameAsString` _fsm_state)))
  (switch `/Game/Blueprints/Characters/MainChar/DF_MC_FSM_States` _fsm_state
    (:`NewEnumerator4`
      (`self.FSMChangeState` "NewEnumerator2" :!label _label)
      (set `MovementComponent.Velocity` (0.0 0.0 0.0) (`self.CharacterMovement`)))
    (:`NewEnumerator5`
      (goto _label))
    (:`NewEnumerator6`
      (if (== _returnvalue 0.0) :!label _label_2
        (goto _label)
        (else
          (set `self.LastMoveInputValue` _returnvalue)
          (`self.FSMChangeState` "NewEnumerator3"))))
    (:`NewEnumerator7`
      (goto _label_2))
    (:`NewEnumerator11`
      (if (`|GetInputActionValue`)
        (`self.FSMChangeState` "NewEnumerator8")
        (else
          (`self.FSMChangeState` "NewEnumerator2"))))
    (:`NewEnumerator12`
      (goto _label))
    (:`NewEnumerator13`
      (goto _label_2))
    (:`NewEnumerator14`
      (`self.FSMChangeState` "NewEnumerator10" :!label _label_3))
    (:`NewEnumerator15`
      (`CharacterMovementComponent.AddForce` (`self.CharacterMovement`) (`KismetMathLibrary.MakeVector` (* (`|GetInputActionValue`) (`self.DoubleJumpLatStrength`)) 0.0 300000.0))
      (goto _label_3))))

(fn `FSMChangeState`
  (params (NewState :type "/Game/Blueprints/Characters/MainChar/DF_MC_FSM_States Enum" :default "NewEnumerator0"))
  (bind _sprite (`self.Sprite`))
  (if (not (`|EnumEquality` NewState (`self.FSM_State`)))
    (`KismetSystemLibrary.PrintString` (`KismetStringLibrary.Concat_StrStr` "DTATE CHANGED : " (`|GetEnumeratorNameAsString` NewState)) true true (struct :`R` 0.178459 :`G` 1.0 :`B` 0.142727 :`A` 1.0))
    (bind _output_get (set `self.FSM_State` NewState))
    (`PaperFlipbookComponent.SetFlipbook` _sprite (select `/Game/Blueprints/Characters/MainChar/DF_MC_FSM_States` _output_get :`NewEnumerator0` "/Game/2DAnims/MainChar/Anim_Prota_conmono/IDLE/MC_M_IDLE.MC_M_IDLE" :`NewEnumerator1` "/Game/2DAnims/MainChar/Anim_Prota_conmono/CORRER/MC_M_RUN.MC_M_RUN" :`NewEnumerator2` "/Game/2DAnims/MainChar/Anim_Prota_sinmono/IDLE_sinmono/MC_FSM_Idle.MC_FSM_Idle" :`NewEnumerator3` "/Game/2DAnims/MainChar/Anim_Prota_sinmono/RUN_sinmono/MC_FSM_RUN.MC_FSM_RUN" :`NewEnumerator4` "/Game/2DAnims/MainChar/Anim_Prota_sinmono/ESQUIVAFONDO_sinmono/MC_FSM_DodgeStatic.MC_FSM_DodgeStatic" :`NewEnumerator5` "/Game/2DAnims/MainChar/Anim_Prota_sinmono/FRENADA_sinmono/MC_FSM_Stop.MC_FSM_Stop" :`NewEnumerator6` "/Game/2DAnims/MainChar/Anim_Prota_sinmono/FRENADAGIRO_sinmono/MC_FSM_Rotate.MC_FSM_Rotate" :`NewEnumerator7` "/Game/2DAnims/MainChar/Anim_Prota_sinmono/ESQUIVALATERALtoRUN_sinmono/MC_FSM_DodgeRunToRun.MC_FSM_DodgeRunToRun" :`NewEnumerator8` "/Game/2DAnims/MainChar/Anim_Prota_sinmono/IDLECOMBATE_sinmono/MC_FSM_IdleCombat.MC_FSM_IdleCombat" :`NewEnumerator10` "/Game/2DAnims/MainChar/Anim_Prota_sinmono/CAIDALIBRE_sinmono/MC_FSM_Fall.MC_FSM_Fall" :`NewEnumerator11` "/Game/2DAnims/MainChar/Anim_Prota_sinmono/PARRY_sinmono/MC_FSM_Parry.MC_FSM_Parry" :`NewEnumerator12` "/Game/2DAnims/MainChar/Anim_Prota_sinmono/ATERRIZAtoIDLE_sinmono/MC_FSM_VertLandToIdle.MC_FSM_VertLandToIdle" :`NewEnumerator13` "/Game/2DAnims/MainChar/Anim_Prota_sinmono/ATERRIZAJEtoRUN_sinmono/MC_FSM_LandToRun.MC_FSM_LandToRun" :`NewEnumerator14` "/Game/2DAnims/MainChar/Anim_Prota_sinmono/SALTOINICIO_sinmono/MC_FSM_JumpStart.MC_FSM_JumpStart" :`NewEnumerator15` "/Game/2DAnims/MainChar/Anim_Prota_sinmono/DOBLESALTO_sinmono/MC_FSM_DoubleJump.MC_FSM_DoubleJump" :!type "PaperFlipbook Object Reference"))
    (switch `/Game/Blueprints/Characters/MainChar/DF_MC_FSM_States` (`self.FSM_State`)
      (:`NewEnumerator0`
        (`PaperFlipbookComponent.SetLooping` _sprite true :!label _label)
        (`PaperFlipbookComponent.SetLooping` (`self.Sprite`) true)
        (`PaperFlipbookComponent.PlayFromStart` (`self.Sprite`)))
      (:`NewEnumerator1`
        (goto _label))
      (:`NewEnumerator2`
        (goto _label))
      (:`NewEnumerator3`
        (goto _label))
      (:`NewEnumerator4`
        (`PaperFlipbookComponent.SetLooping` (`self.Sprite`) false :!label _label_2))
      (:`NewEnumerator5`
        (goto _label_2))
      (:`NewEnumerator6`
        (goto _label_2))
      (:`NewEnumerator7`
        (goto _label_2))
      (:`NewEnumerator8`
        (goto _label))
      (:`NewEnumerator10`
        (goto _label))
      (:`NewEnumerator11`
        (goto _label_2))
      (:`NewEnumerator12`
        (goto _label_2))
      (:`NewEnumerator13`
        (goto _label_2))
      (:`NewEnumerator14`
        (goto _label_2))
      (:`NewEnumerator15`
        (goto _label_2)))))

(fn `FSMUpdateState`
  (bind _charactermovement (`self.CharacterMovement`))
  (bind _charactermovement_2 (`self.CharacterMovement`))
  (bind _returnvalue_x (`KismetMathLibrary.BreakVector` (`SceneComponent.K2_GetComponentScale` (`self.Sprite`))))
  (bind (_velocity_x _velocity_y _velocity_z) (`KismetMathLibrary.BreakVector` (`MovementComponent.Velocity` _charactermovement)))
  (bind (_velocity_x_2 _velocity_y_2 _velocity_z_2) (`KismetMathLibrary.BreakVector` (`MovementComponent.Velocity` _charactermovement_2)))
  (switch `/Game/Blueprints/Characters/MainChar/DF_MC_FSM_States` (`self.FSM_State`)
    (:`NewEnumerator7`
      (set `MovementComponent.Velocity` (`KismetMathLibrary.MakeVector` (* _returnvalue_x (`self.DodgeMoveSpeed`)) 0.0 _velocity_z_2) _charactermovement_2))
    (:`NewEnumerator10`
      (if (== _velocity_z 0.0)
        (`/Engine/EditorBlueprintResources/StandardMacros.CompareFloat` (`|GetInputActionValue`)
          (:`>`
            (`self.FSMChangeState` "NewEnumerator13" :!label _label))
          (:`==`
            (`self.FSMChangeState` "NewEnumerator12"))
          (:`<`
            (goto _label)))
        (set `self.CanDoubleJump` true)))
    (:`NewEnumerator15`
      (set `MovementComponent.Velocity` (0.0 0.0 0.0) _charactermovement))))

(fn `GetMonkey`
  (set `self.HasMonkey` true)
  (`SceneComponent.SetVisibility` (`self.MonkeySprite`) true false)
  (`/Game/Blueprints/Characters/Monkey/MK_MonkeyChar.GetMeBack` (`self.MonkeyReference`)))

(fn `InitMappingContext`
  (`EnhancedInputSubsystemInterface.AddMappingContext` (pcsubsystem `EnhancedInputLocalPlayerSubsystem` (`GameplayStatics.GetPlayerController` 0)) "/Game/Inputs/MainChar/IMP_MC_Context.IMP_MC_Context" 0 (struct)))

(fn `ThrowMonkey`
  (bind (_returnvalue_x _returnvalue_y) (`KismetMathLibrary.BreakVector2D` (`|GetInputActionValue`)))
  (if (`self.HasMonkey`)
    (`/Game/Blueprints/Characters/Monkey/MK_MonkeyChar.ThrowMe` (`self.MonkeyReference`) (`KismetMathLibrary.MakeVector` _returnvalue_x 0.0 (* _returnvalue_y -1.0)) (`self.MonkeyThrowStrength`) (`SceneComponent.K2_GetComponentLocation` (`self.MonkeySprite`)))
    (set `self.HasMonkey` false)
    (`SceneComponent.SetVisibility` (`self.MonkeySprite`) false false)
    (`SceneComponent.SetVisibility` (`/Game/Blueprints/Characters/Monkey/MK_MonkeyChar.DefaultSceneRoot` (`self.MonkeyReference`)) true true)))

(fn `UpdateSpriteScale`
  (bind (_x _y) (`KismetMathLibrary.BreakVector2D` (1.0 -1.0)))
  (bind _velocity_x (`KismetMathLibrary.BreakVector` (`MovementComponent.Velocity` (`self.CharacterMovement`))))
  (if (not (== _velocity_x 0.0))
    (`SceneComponent.SetWorldScale3D` (`self.Sprite`) (`KismetMathLibrary.MakeVector` (select `bool` (< _velocity_x 0.0) :`false` _x :`true` _y) 1.0 1.0))))

(fn `UserConstructionScript`)