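; Generic enemy Blueprint that runs a timed attack cycle the player can block to stun it.
; After a start delay, BeginPlay loops an attack sequence, with Sequencer events driving the state machine through wait, attack, damage window, recoil and idle.
; During the damage window, Tick polls the player's BeingAttacked and switches to Stunned on true, which recoil respects.
; Each state change recolors the placeholder body and prints debug text.
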(event `self.ReceiveBeginPlay`
  (bind _returnvalue (`GameplayStatics.GetActorOfClass` "/Game/Blueprints/Characters/MainChar/DF_PlayerPaperBP.DF_PlayerPaperBP_C"))
  (set `self.RefToPlayer` _returnvalue)
  (`KismetSystemLibrary.Delay` 5.0)
  (`self.PlayAttackSequence` :!label _label)
  (`KismetSystemLibrary.Delay` 10.0)
  (goto _label))

(event `self.ReceiveTick`
  (params (DeltaSeconds :type "Float (single-precision)"))
  (switch `/Game/Blueprints/Characters/Enemies/Generic/DF_GE_FSMStates` (`self.FSMState`)
    (:`NewEnumerator3`
      (`self.UpdateDamageWindow`))))

(event `ToWait`
  (`self.ChangeFSMState` "NewEnumerator1"))

(event `ToAttack`
  (`self.ChangeFSMState` "NewEnumerator2"))

(event `ToDmgWindow`
  (`self.ChangeFSMState` "NewEnumerator3"))

(event `ToRecoil`
  (if (`|EnumInequality` (`self.FSMState`) "NewEnumerator5")
    (`self.ChangeFSMState` "NewEnumerator4")))

(event `ToIdle`
  (`self.ChangeFSMState` "NewEnumerator0"))

(fn `ChangeFSMState`
  (params (newState :type "/Game/Blueprints/Characters/Enemies/Generic/DF_GE_FSMStates Enum" :default "NewEnumerator0"))
  (bind _output_get (set `self.FSMState` newState))
  (`PrimitiveComponent.SetMaterial` (`self.TempBody`) 0 (select `/Game/Blueprints/Characters/Enemies/Generic/DF_GE_FSMStates` _output_get :`NewEnumerator0` "/Game/Materials/Unlit/Mat_Unlit_White.Mat_Unlit_White" :`NewEnumerator1` "/Game/Materials/Unlit/Mat_Unlit_Green.Mat_Unlit_Green" :`NewEnumerator2` "/Game/Materials/Unlit/Mat_Unlit_Blue.Mat_Unlit_Blue" :`NewEnumerator3` "/Game/Materials/Unlit/Mat_Unlit_Red.Mat_Unlit_Red" :`NewEnumerator4` "/Game/Materials/Unlit/Mat_Unlit_Green.Mat_Unlit_Green" :`NewEnumerator5` "/Game/Materials/Unlit/Mat_Unlit_Yellow.Mat_Unlit_Yellow" :!type "MaterialInterface Object Reference"))
  (`KismetSystemLibrary.PrintString` (`KismetStringLibrary.Concat_StrStr` "ENEMY NEW STATE : " (`|GetEnumeratorNameAsString` _output_get)) true true (struct :`R` 1.0 :`G` 0.214584 :`A` 1.0) 5.0))

(fn `PlayAttackSequence`
  (`ActorSequenceComponent.PlaySequence` (`self.AttackSequence`)))

(fn `UpdateDamageWindow`
  (bind _hitsuccess (`/Game/Blueprints/Characters/MainChar/DF_PlayerPaperBP.BeingAttacked` (`self.RefToPlayer`)))
  (if _hitsuccess
    (`KismetSystemLibrary.PrintString` "ATTACK BLOCKED!" true true (struct :`R` 0.445232 :`G` 1.0 :`A` 1.0))
    (`self.ChangeFSMState` "NewEnumerator5")))

(fn `UserConstructionScript`)